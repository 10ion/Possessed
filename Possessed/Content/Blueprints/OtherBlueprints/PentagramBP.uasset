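; PentagramBP is a pentagram actor with a box trigger that destroys itself on overlap once the Gameplay game mode reports no collectables left.
; Its AddItem event also destroys it directly.
; Leaving the box disables its input for player 0 after a FirstPersonCharacter cast, then enables it for player 1 if a chained FirstPersonCharacter1 cast succeeds.
; A branch enabling input for both players is unwired.
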(event `Add Item`
  (`self.K2_DestroyActor`))

(event `Key|E`
  (params (Key :type "Key Structure")))

(event `self.Box.OnComponentBeginOverlap`
  (params (OverlappedComponent :type "PrimitiveComponent Object Reference") (OtherActor :type "Actor Object Reference") (OtherComp :type "PrimitiveComponent Object Reference") (OtherBodyIndex :type Integer) (bFromSweep :type Boolean) (SweepResult :type "HitResult Structure (by ref)"))
  (bind _asgameplay (cast `/Game/Blueprints/Gamemodes/Gameplay` (`GameplayStatics.GetGameMode`)))
  (if (== (`/Game/Blueprints/Gamemodes/Gameplay.CollectablesLeft` _asgameplay) 0)
    (`self.K2_DestroyActor`)))

(event `self.Box.OnComponentEndOverlap`
  (params (OverlappedComponent :type "PrimitiveComponent Object Reference") (OtherActor :type "Actor Object Reference") (OtherComp :type "PrimitiveComponent Object Reference") (OtherBodyIndex :type Integer))
  (cast `/Game/Blueprints/Pawns/FirstPersonCharacter` OtherActor)
  (`self.DisableInput` (`GameplayStatics.GetPlayerController` 0))
  (cast `/Game/Blueprints/Pawns/FirstPersonCharacter1` OtherActor)
  (`self.EnableInput` (`GameplayStatics.GetPlayerController` 1)))

(fn `UserConstructionScript`)