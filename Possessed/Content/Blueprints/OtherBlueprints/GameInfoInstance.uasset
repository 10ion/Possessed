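; Game instance that manages the game's menus and multiplayer session flow, and overrides the network version on init.
; Menu events show the main, host, options and server widgets, caching all but the server menu.
; LobbyLaunch creates a session and opens the lobby as a listen server, while other events join or destroy sessions.
; Session, network and travel failures print through DisplayError; the loading widget is created but never displayed here.
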(event `self.ReceiveInit`
  (`KismetSystemLibrary.ExecuteConsoleCommand` "NetworkVersionOverride 12345" (`GameplayStatics.GetPlayerController` 0)))

(event `ShowLoading`
  (bind _returnvalue (`|CreateWidget` "/Game/Blueprints/Widgets/LoadingScreen.LoadingScreen_C" (`GameplayStatics.GetPlayerController` 0)))
  (set `self.LoadingWD` _returnvalue))

(event `self.HandleNetworkError`
  (params (FailureType :type "ENetworkFailure Enum" :default "NetDriverAlreadyExists") (bIsServer :type Boolean))
  (if bIsServer
    _
    (else
      _))
  (`self.DisplayError` (`self.NetErrorToString` FailureType)))

(event `MainMenueShow`
  (bind _returnvalue (`GameplayStatics.GetPlayerController` 0))
  ;[1 1 1] Main Menue
  (`/Engine/EditorBlueprintResources/StandardMacros.IsValid` (`self.MainMenueWD`)
    (:`Is Valid`
      _)
    (:`Is Not Valid`
      (bind _returnvalue_2 (`|CreateWidget` "/Game/Blueprints/Widgets/MainMenueUI.MainMenueUI_C" _returnvalue))
      (set `self.MainMenueWD` _returnvalue_2)))
  (`UserWidget.AddToViewport` (cast `/Game/Blueprints/Widgets/MainMenueUI` (`self.MainMenueWD`) :!pure true) 0)
  (set `PlayerController.bShowMouseCursor` true _returnvalue))

(event `self.HandleTravelError`
  (params (FailureType :type "ETravelFailure Enum" :default "NoLevel"))
  (`self.DisplayError` (`self.TravelErrorToString` FailureType)))

(event `Join Sever`
  (params (SessionToJoin :type "BlueprintSessionResult Structure"))
  (set `self.Session to Join` SessionToJoin)
  (`JoinSessionCallbackProxy.JoinSession` (`GameplayStatics.GetPlayerController` 0) SessionToJoin
    (:`OnFailure`
      (`self.DisplayError` "Failed To Join Session, Please Try Again."))))

(event `DestroySessionCaller`
  (params (PlayerController :type "PlayerController Object Reference"))
  (`DestroySessionCallbackProxy.DestroySession` PlayerController))

(event `HostMenue`
  (bind _returnvalue (`GameplayStatics.GetPlayerController` 0))
  ;[1 1 1] HostMenue
  (`/Engine/EditorBlueprintResources/StandardMacros.IsValid` (`self.HostMenueWD`)
    (:`Is Valid`
      _)
    (:`Is Not Valid`
      (bind _returnvalue_2 (`|CreateWidget` "/Game/Blueprints/Widgets/HostMenue.HostMenue_C" _returnvalue))
      (set `self.HostMenueWD` _returnvalue_2)))
  (`UserWidget.AddToViewport` (`self.HostMenueWD`) 0)
  (set `PlayerController.bShowMouseCursor` true _returnvalue))

(event `LobbyLaunch`
  (params (`Number of Players` :type Integer) (`Is Local` :type Boolean) (`Server Name` :type Text))
  ;[1 1 1] Add Lobby
  (bind _output_get (set `self.Number Of Players` `Number of Players`))
  (set `self.Server Name` `Server Name`)
  (`self.ShowLoading`)
  (`CreateSessionCallbackProxy.CreateSession` (`GameplayStatics.GetPlayerController` 0) _output_get `Is Local`
    (:`OnSuccess`
      (`GameplayStatics.OpenLevelBySoftObjectPtr` "/Game/Maps/LobbyWorld.LobbyWorld" true "listen"))
    (:`OnFailure`
      (`self.DisplayError` "Failed to Create Session, Please Try Again."))))

(event `ServerMenue`
  (bind _returnvalue (`|CreateWidget` "/Game/Blueprints/Widgets/ServerMenue.ServerMenue_C" (`GameplayStatics.GetPlayerController` 0)))
  (`UserWidget.AddToViewport` _returnvalue 0))

(event `OptionsMenue`
  (bind _returnvalue (`GameplayStatics.GetPlayerController` 0))
  ;[1 1 1] Options Menue
  (`/Engine/EditorBlueprintResources/StandardMacros.IsValid` (`self.OptioinsMenueWD`)
    (:`Is Valid`
      _)
    (:`Is Not Valid`
      (bind _returnvalue_2 (`|CreateWidget` "/Game/Blueprints/Widgets/OptionsMenue.OptionsMenue_C" _returnvalue))
      (set `self.OptioinsMenueWD` _returnvalue_2)))
  (`UserWidget.AddToViewport` (`self.OptioinsMenueWD`) 0)
  (set `PlayerController.bShowMouseCursor` true _returnvalue))

(fn `NetErrorToString`
  (params (FailureType :type "ENetworkFailure Enum" :default "NetDriverAlreadyExists"))
  (returns (OutString :type String))
  (return (`|GetEnumeratorNameAsString` FailureType)))

(fn `OnRep_PlayerTaken`)

(fn `TravelErrorToString`
  (params (FailureType :type "ETravelFailure Enum" :default "NoLevel"))
  (returns (OutString :type String))
  (return (`|GetEnumeratorNameAsString` FailureType)))