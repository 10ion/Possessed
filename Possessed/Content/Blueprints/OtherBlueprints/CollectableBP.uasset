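; CollectableBP is a pickup actor that counts down the remaining collectables when its Box is overlapped.
; Any overlapping actor decrements CollectablesLeft on the Gameplay game mode, adds a CollectableWidget to the viewport, then destroys the pickup.
; End overlap by a FirstPersonCharacter calls DisableInput for player controller 0, while the EnableInput branches for both players are unconnected and never run.
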(event `Key|E`
  (params (Key :type "Key Structure")))

(event `self.Box.OnComponentBeginOverlap`
  (params (OverlappedComponent :type "PrimitiveComponent Object Reference") (OtherActor :type "Actor Object Reference") (OtherComp :type "PrimitiveComponent Object Reference") (OtherBodyIndex :type Integer) (bFromSweep :type Boolean) (SweepResult :type "HitResult Structure (by ref)"))
  (bind _asgameplay (cast `/Game/Blueprints/Gamemodes/Gameplay` (`GameplayStatics.GetGameMode`)))
  (bind _result (`/Engine/EditorBlueprintResources/StandardMacros.DecrementInt` (`/Game/Blueprints/Gamemodes/Gameplay.CollectablesLeft` _asgameplay))
    (:`  `
      (set `/Game/Blueprints/Gamemodes/Gameplay.CollectablesLeft` _result _asgameplay)
      (bind _returnvalue (`|CreateWidget` "/Game/Blueprints/Widgets/CollectableWidget.CollectableWidget_C"))
      (`UserWidget.AddToViewport` _returnvalue 0)
      (`self.K2_DestroyActor`))))

(event `self.Box.OnComponentEndOverlap`
  (params (OverlappedComponent :type "PrimitiveComponent Object Reference") (OtherActor :type "Actor Object Reference") (OtherComp :type "PrimitiveComponent Object Reference") (OtherBodyIndex :type Integer))
  (cast `/Game/Blueprints/Pawns/FirstPersonCharacter` OtherActor)
  (`self.DisableInput` (`GameplayStatics.GetPlayerController` 0)))

(fn `UserConstructionScript`)