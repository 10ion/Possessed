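; Maxtest is an actor, apparently a test, that bounces up and down along Z at constant speed between fixed lower and upper height limits.
; Tick adds a frame-time-scaled step to the current height, clamps it and sets the location, keeping X and Y.
; Reaching either limit sets the IsUp flag that picks direction, with true meaning descent despite the name.
; The overlap, hit and custom events are empty stubs.
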(event `self.ReceiveBeginPlay`)

(event `self.ReceiveTick`
  (params (DeltaSeconds :type "Float (single-precision)"))
  (bind (_returnvalue_x _returnvalue_y _returnvalue_z) (`KismetMathLibrary.BreakVector` (`self.K2_GetActorLocation`)))
  (bind _returnvalue (`KismetMathLibrary.FClamp` (+ (* DeltaSeconds (select `bool` (`self.IsUp`) :`false` 299.0 :`true` -299.0 :!type "Float (single-precision)")) _returnvalue_z) 40.0 1111.0))
  (bind _returnvalue_2 (== _returnvalue 1111.0))
  (if _returnvalue_2
    (set `self.IsUp` _returnvalue_2)
    (elif (== _returnvalue 40.0)
      (set `self.IsUp` false)))
  (`self.K2_SetActorLocation` (`KismetMathLibrary.MakeVector` _returnvalue_x _returnvalue_y _returnvalue)))

(event `OnActorBeginOverlap_Event_0`
  (params (OverlappedActor :type "Actor Object Reference") (OtherActor :type "Actor Object Reference")))

(event `self.Cube.OnComponentHit`
  (params (HitComponent :type "PrimitiveComponent Object Reference") (OtherActor :type "Actor Object Reference") (OtherComp :type "PrimitiveComponent Object Reference") (NormalImpulse :type "Vector Structure") (Hit :type "HitResult Structure (by ref)")))

(event `CustomEvent`
  (params (DeltaSeconds :type "Float (double-precision)")))

(fn `UserConstructionScript`)