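; BP_Pickup is a world item the player collects with E, configured from a data table row that sets its info and mesh at construction.
; An interaction collider shows a "[E] Name" nameplate widget and enables input while a FirstPersonCharacter1 overlaps, reversing both on exit.
; Pressing E passes the item and quantity to the overlapping GamePlayController's AddItem, then has that controller destroy the pickup if it succeeds.
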(event `self.ReceiveBeginPlay`
  (bind _aswg_pickup_nameplate (cast `/Game/Blueprints/Widgets/WG_Pickup_Nameplate` (`WidgetComponent.GetUserWidgetObject` (`self.NamePlate`))))
  (`TextBlock.SetText` (`/Game/Blueprints/Widgets/WG_Pickup_Nameplate.NameText` _aswg_pickup_nameplate) (`KismetTextLibrary.Conv_StringToText` (`KismetStringLibrary.Concat_StrStr` "[E]" (`KismetStringLibrary.Conv_NameToString` (`.Name_9_78FD7AC849FA6952B32C41A665950DF6` (break `/Game/Blueprints/OtherBlueprints/ST_Item` (`self.Information`))))))))

(event `self.InteractionCollider.OnComponentBeginOverlap`
  (params (OverlappedComponent :type "PrimitiveComponent Object Reference") (OtherActor :type "Actor Object Reference") (OtherComp :type "PrimitiveComponent Object Reference") (OtherBodyIndex :type Integer) (bFromSweep :type Boolean) (SweepResult :type "HitResult Structure (by ref)"))
  (if (`KismetMathLibrary.ClassIsChildOf` (`GameplayStatics.GetObjectClass` OtherActor) "/Game/Blueprints/Pawns/FirstPersonCharacter1.FirstPersonCharacter1_C")
    (`SceneComponent.SetVisibility` (`self.NamePlate`) true false)
    (`self.EnableInput` (cast `/Game/Blueprints/Controllers/GamePlayController` (`Pawn.GetController` (`Actor.Instigator` OtherActor)) :!pure true))))

(event `self.InteractionCollider.OnComponentEndOverlap`
  (params (OverlappedComponent :type "PrimitiveComponent Object Reference") (OtherActor :type "Actor Object Reference") (OtherComp :type "PrimitiveComponent Object Reference") (OtherBodyIndex :type Integer))
  (if (`KismetMathLibrary.ClassIsChildOf` (`GameplayStatics.GetObjectClass` OtherActor) "/Game/Blueprints/Pawns/FirstPersonCharacter1.FirstPersonCharacter1_C")
    (`SceneComponent.SetVisibility` (`self.NamePlate`) false false)
    (`self.DisableInput` (cast `/Game/Blueprints/Controllers/GamePlayController` (`Pawn.GetController` (`Actor.Instigator` OtherActor)) :!pure true))
    (`KismetSystemLibrary.PrintString` (`KismetSystemLibrary.GetDisplayName` (cast `/Game/Blueprints/Controllers/GamePlayController` (`Pawn.GetController` (`Actor.Instigator` (stale `self.InteractionCollider.OnComponentBeginOverlap` OtherActor))) :!pure true)) true true (struct :`R` 1.0 :`G` 0.045265 :`B` 0.121616 :`A` 1.0))))

(event `Key|E`
  (params (Key :type "Key Structure"))
  (:`Pressed`
    (bind _asgame_play_controller (cast `/Game/Blueprints/Controllers/GamePlayController` (`Pawn.GetController` (`Actor.Instigator` (stale `self.InteractionCollider.OnComponentBeginOverlap` OtherActor))) :!pure true))
    (bind _itemadded (`/Game/Blueprints/Controllers/GamePlayController.AddItem` _asgame_play_controller (`.Quantity_18_57DBDB0C4CCC08681896CD96DD6798C1` (break `/Game/Blueprints/OtherBlueprints/ST_Item` (`self.Information`))) (`self.Information`)))
    (if _itemadded
      (`/Game/Blueprints/Controllers/GamePlayController.DestroyObject` _asgame_play_controller self)
      (else
        (`KismetSystemLibrary.PrintString` (`KismetSystemLibrary.GetDisplayName` _asgame_play_controller))))))

(fn `UserConstructionScript`
  (bind (_datatable _rowname) (break `DataTableRowHandle` (`self.Item`)))
  (bind _returnvalue (`|GetDataTableRow` _datatable _rowname)
    (:`then`
      (set `self.Information` _returnvalue)
      (`StaticMeshComponent.SetStaticMesh` (`self.Model`) (`.Model_20_7003C297461B8273CE0068A788F23FCC` (break `/Game/Blueprints/OtherBlueprints/ST_Item` (`self.Information`)))))))