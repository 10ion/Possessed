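; Blueprint function library for the player inventory, covering UI setup and adding, removing and finding items.
; InitializeInventory builds a slot-widget grid on the main HUD and loads slot data from GameInfoInstance, or seeds that array when empty.
; Slot widgets hold item data, located through widget searches and scanned by name or emptiness.
; AddItem stacks stackable items or fills an empty slot; RemoveItem passes negative amounts to UpdateQuantity.
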(fn `Add Item`
  (params (ItemToAdd :type "/Game/Blueprints/OtherBlueprints/ST_Item Structure") (QuantityToAdd :type Integer))
  (returns (SuccessfullyAdded :type Boolean))
  (locals (ItemToAddInfoRef :type "/Game/Blueprints/OtherBlueprints/ST_Item Structure") (QuantityToAddRef :type Integer))
  (bind (_name _types _description _icon _model _rarity _quantity _stackable) (break `/Game/Blueprints/OtherBlueprints/ST_Item` (`local.ItemToAddInfoRef`)))
  (set `local.ItemToAddInfoRef` ItemToAdd)
  (set `local.QuantityToAddRef` QuantityToAdd)
  (if _stackable
    (bind (_founditem _amountfound _slot) (`self.ScanForItem` _name))
    (if _founditem
      (`self.UpdateQuantity` _slot (`local.QuantityToAddRef`))
      (return true)
      (else
        _)))
  (bind (_foundemptyslot _slot_2) (`self.ScanForEmptySlot` null))
  (if _foundemptyslot
    (bind _output_get (set `/Game/Blueprints/Widgets/WG_Inventory_Slot.Information` (`local.ItemToAddInfoRef`) _slot_2))
    (`|VariableSetRef` (`.Quantity_18_57DBDB0C4CCC08681896CD96DD6798C1` (break `/Game/Blueprints/OtherBlueprints/ST_Item` _output_get)) (`local.QuantityToAddRef`))
    (`/Game/Blueprints/Widgets/WG_Inventory_Slot.UpdateUI` _slot_2)
    (return true)
    (else
      (return false))))

(fn `GetHUD`
  (returns (HudRef :type "/Game/Blueprints/Widgets/WG_Main_HUD Object Reference"))
  (bind _foundwidgets (`WidgetBlueprintLibrary.GetAllWidgetsOfClass` (`local.__WorldContext`) "/Game/Blueprints/Widgets/WG_Main_HUD.WG_Main_HUD_C"))
  (for _array_element _foundwidgets
    (return _array_element)))

(fn `GetInventoryReference`
  (returns (InventoryRef :type "/Game/Blueprints/Widgets/WG_Inventory Object Reference"))
  (bind _foundwidgets (`WidgetBlueprintLibrary.GetAllWidgetsOfClass` null "/Game/Blueprints/Widgets/WG_Inventory.WG_Inventory_C" false))
  (for _array_element _foundwidgets
    (return _array_element))
  (`KismetSystemLibrary.PrintString` null (`KismetStringLibrary.Concat_StrStr` (`KismetSystemLibrary.GetDisplayName` _array_element) "" "is found on widget")))

(fn `InitializeInventory`
  (params (NumberOfSlots :type Integer) (ScreenAnchors :type "Anchors Structure"))
  (locals (InventoryPanel :type "/Game/Blueprints/Widgets/WG_Inventory Object Reference") (HudRef :type "/Game/Blueprints/Widgets/WG_Main_HUD Object Reference") (NewSlot :type "/Game/Blueprints/Widgets/WG_Inventory_Slot Object Reference") (GameInstanceRef :type "/Game/Blueprints/OtherBlueprints/GameInfoInstance Object Reference"))
  (set `local.HudRef` (`self.GetHUD` null))
  (bind _returnvalue (`|CreateWidget` "/Game/Blueprints/Widgets/WG_Inventory.WG_Inventory_C"))
  (bind _output_get (set `local.InventoryPanel` _returnvalue))
  (bind _returnvalue_2 (`CanvasPanel.AddChildToCanvas` (`/Game/Blueprints/Widgets/WG_Main_HUD.MainPanel` (`local.HudRef`)) _output_get))
  (`CanvasPanelSlot.SetAutoSize` _returnvalue_2 false)
  (`CanvasPanelSlot.SetAnchors` _returnvalue_2 ScreenAnchors)
  (`CanvasPanelSlot.SetOffsets` _returnvalue_2 (make `Margin` 0.0))
  (set `local.GameInstanceRef` (cast `/Game/Blueprints/OtherBlueprints/GameInfoInstance` (`GameplayStatics.GetGameInstance` null) :!pure true))
  (for _index (range NumberOfSlots)
    (bind _returnvalue_3 (`|CreateWidget` "/Game/Blueprints/Widgets/WG_Inventory_Slot.WG_Inventory_Slot_C"))
    (set `local.NewSlot` _returnvalue_3)
    (set `/Game/Blueprints/Widgets/WG_Inventory_Slot.InventoryIndex` _index (`local.NewSlot`))
    (`KismetArrayLibrary.Array_Add` (`/Game/Blueprints/Widgets/WG_Inventory.InventorySlots` (`local.InventoryPanel`)) (`local.NewSlot`))
    (`WrapBox.AddChildToWrapBox` (`/Game/Blueprints/Widgets/WG_Inventory.SlotsPanel` (`local.InventoryPanel`)) (`local.NewSlot`)))
  (if (> (`KismetArrayLibrary.Array_Length` (`/Game/Blueprints/OtherBlueprints/GameInfoInstance.InventoryItems` (`local.GameInstanceRef`))) 0)
    (for (_array_element _array_index) (`/Game/Blueprints/Widgets/WG_Inventory.InventorySlots` (`local.InventoryPanel`))
      (set `/Game/Blueprints/Widgets/WG_Inventory_Slot.Information` (`|GetArrayItem` (`/Game/Blueprints/OtherBlueprints/GameInfoInstance.InventoryItems` (`local.GameInstanceRef`)) _array_index) _array_element))
    (else
      (for _ (`/Game/Blueprints/Widgets/WG_Inventory.InventorySlots` (`local.InventoryPanel`))
        (`KismetArrayLibrary.Array_Add` (`/Game/Blueprints/OtherBlueprints/GameInfoInstance.InventoryItems` (`local.GameInstanceRef`)))))))

(fn `RemoveItem`
  (params (ItemToRemove :type "/Game/Blueprints/OtherBlueprints/ST_Item Structure") (QuantityToRemove :type Integer :default 1))
  (returns (SuccessfullyRemoved :type Boolean))
  (bind (_founditem _amountfound _slot) (`self.ScanForItem` (`.Name_9_78FD7AC849FA6952B32C41A665950DF6` (break `/Game/Blueprints/OtherBlueprints/ST_Item` ItemToRemove))))
  (if _founditem
    (`self.UpdateQuantity` _slot (* QuantityToRemove -1))
    (return true)
    (else
      (return false))))

(fn `ScanForEmptySlot`
  (returns (FoundEmptySlot :type Boolean) (Slot :type "/Game/Blueprints/Widgets/WG_Inventory_Slot Object Reference"))
  (for _array_element (`/Game/Blueprints/Widgets/WG_Inventory.InventorySlots` (`self.GetInventoryReference` null))
    (if (== (`.Name_9_78FD7AC849FA6952B32C41A665950DF6` (break `/Game/Blueprints/OtherBlueprints/ST_Item` (`/Game/Blueprints/Widgets/WG_Inventory_Slot.Information` _array_element))) "None")
      (return true _array_element)))
  (return false null))

(fn `ScanForItem`
  (params (ItemToCheckFor :type Name))
  (returns (FoundItem :type Boolean) (AmountFound :type Integer) (Slot :type "/Game/Blueprints/Widgets/WG_Inventory_Slot Object Reference") (ItemInfo :type "/Game/Blueprints/OtherBlueprints/ST_Item Structure"))
  (for _array_element (`/Game/Blueprints/Widgets/WG_Inventory.InventorySlots` (`self.GetInventoryReference` null))
    (bind _information (`/Game/Blueprints/Widgets/WG_Inventory_Slot.Information` _array_element))
    (bind (_name _types _description _icon _model _rarity _quantity) (break `/Game/Blueprints/OtherBlueprints/ST_Item` _information))
    (if (== _name ItemToCheckFor)
      (return true _quantity _array_element _information)))
  (return false 0 null))

(fn `UpdateQuantity`
  (params (SlotToUpdate :type "/Game/Blueprints/Widgets/WG_Inventory_Slot Object Reference") (QuantityToAdd :type Integer))
  (locals (Slot :type "/Game/Blueprints/Widgets/WG_Inventory_Slot Object Reference") (`Final Quantity` :type Integer))
  (bind _output_get (set `local.Slot` SlotToUpdate))
  (bind _output_get_2 (set `local.Final Quantity` (+ (`.Description_22_CF3BCB14443137FBDD76E2992408CE80` (break `/Game/Blueprints/OtherBlueprints/ST_Item` (`/Game/Blueprints/Widgets/WG_Inventory_Slot.Information` _output_get))) QuantityToAdd)))
  (if (<= _output_get_2 0)
    (set `/Game/Blueprints/Widgets/WG_Inventory_Slot.Information` (struct) (`local.Slot`))
    (`/Game/Blueprints/Widgets/WG_Inventory_Slot.UpdateUI` (`local.Slot`))
    (else
      (`|VariableSetRef` (`.Quantity_18_57DBDB0C4CCC08681896CD96DD6798C1` (break `/Game/Blueprints/OtherBlueprints/ST_Item` (`/Game/Blueprints/Widgets/WG_Inventory_Slot.Information` (`local.Slot`)))) (`local.Final Quantity`))
      (`/Game/Blueprints/Widgets/WG_Inventory_Slot.UpdateUI` (`local.Slot`)))))