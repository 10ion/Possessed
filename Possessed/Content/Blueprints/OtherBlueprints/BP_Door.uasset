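; BP_Door is an interactable door that swings open and closed.
; Interact flips the Open flag and plays or reverses Door_Timeline, whose track lerps the Door component's relative yaw between closed and a quarter turn.
; InteractState always returns false, and Interact still prints a debug string.
; A location lerp on the same timeline track is left unused.
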(event `/Game/Blueprints/OtherBlueprints/BP_Interact_Interface.Interact`
  (`KismetSystemLibrary.PrintString` "1")
  (if (`self.Open`)
    (set `self.Open` false)
    (bind (_direction _newtrack_0) (`Timeline|Door_Timeline` :!via `Reverse` :!label _label)
      (:`Update`
        (`SceneComponent.K2_SetRelativeLocationAndRotation` (`self.Door`) (0.0 0.0 0.0) (`KismetMathLibrary.MakeRotator` 0.0 0.0 (`KismetMathLibrary.Lerp` 0.0 90.0 _newtrack_0)) false false)))
    (else
      (set `self.Open` true)
      (goto _label))))

(fn `InteractState`
  (returns (InteractState :type Boolean))
  (return false))

(fn `UserConstructionScript`)