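; EnemyCube is an enemy actor that is destroyed by laser hits and explodes.
; Overlapping a LaserCollision actor destroys it immediately, and Tick also destroys it when Hitpoints is zero or below.
; On destruction it spawns Blueprint_Effect_Explosion at the Cube component's world location.
; The Hitpoints decrement is disconnected, so laser hits bypass the hitpoint count.
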(event `self.ReceiveActorBeginOverlap`
  (params (OtherActor :type "Actor Object Reference"))
  (cast `/Game/Blueprints/OtherBlueprints/LaserCollision` OtherActor)
  (`self.K2_DestroyActor`))

(event `self.ReceiveTick`
  (params (DeltaSeconds :type "Float (single-precision)"))
  (`/Engine/EditorBlueprintResources/StandardMacros.CompareInt` (`self.Hitpoints`)
    (:`==`
      _)
    (:`<`
      _))
  (`self.K2_DestroyActor`))

(event `self.ReceiveDestroyed`
  (`|SpawnActorFromClass` "/Game/StarterContent/Blueprints/Blueprint_Effect_Explosion.Blueprint_Effect_Explosion_C" (`KismetMathLibrary.Conv_VectorToTransform` (`SceneComponent.K2_GetComponentLocation` (`self.Cube`))) "Undefined" "OverrideRootScale" null null))

(fn `UserConstructionScript`)