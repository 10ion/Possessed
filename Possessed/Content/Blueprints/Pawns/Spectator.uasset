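; Spectator pawn that flies freely, switching its CharacterMovement to Flying mode on BeginPlay.
; MoveForward adds movement along the camera's forward vector, as does MoveRight, which uses that forward vector instead of the right vector and prints its axis value.
; Turn adds controller yaw, while LookUp pitches the camera component directly through local rotation.
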(event `self.ReceiveBeginPlay`
  (`CharacterMovementComponent.SetMovementMode` (`self.CharacterMovement`) "MOVE_Flying" 0))

(event `InputAxis|MoveForward` :consume false :overrideparent false
  (params (AxisValue :type "Float (single-precision)"))
  (`self.AddMovementInput` (`SceneComponent.GetForwardVector` (`self.Camera`)) AxisValue))

(event `InputAxis|MoveRight` :consume false :overrideparent false
  (params (AxisValue :type "Float (single-precision)"))
  (`self.AddMovementInput` (`SceneComponent.GetForwardVector` (`self.Camera`)) AxisValue)
  (`KismetSystemLibrary.PrintString` (`KismetStringLibrary.Conv_DoubleToString` AxisValue)))

(event `InputAxis|Turn` :overrideparent false
  (params (AxisValue :type "Float (single-precision)"))
  (`self.AddControllerYawInput` AxisValue))

(event `InputAxis|LookUp` :overrideparent false
  (params (AxisValue :type "Float (single-precision)"))
  (bind _result (`/Engine/EditorBlueprintResources/StandardMacros.NegateFloat` AxisValue)
    (:`  `
      (`SceneComponent.K2_AddLocalRotation` (`self.Camera`) (`KismetMathLibrary.MakeRotator` 0.0 _result) false false))))

(fn `UserConstructionScript`)