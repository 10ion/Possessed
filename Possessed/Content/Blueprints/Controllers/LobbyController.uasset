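; Player controller for the multiplayer lobby, handling each player's menu, profile, character choice and chat.
; It persists player settings to a save slot and reports them to the Lobby game mode, which claims and frees characters through a shared availability array.
; Incoming updates refresh the lobby widget, while chat fans out through every LobbyController.
; It also shows the loading screen and destroys the session on kick or EndPlay.
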(event `InitialSetup`
  (`self.SaveGameCheck`)
  (`self.CallUpdate` (`self.PlayerSettings`)))

(event `SetLobbyMenue`
  (params (ServerName :type Text))
  (set `self.bShowMouseCursor` true)
  (bind _returnvalue (`|CreateWidget` "/Game/Blueprints/Widgets/LobbyUi.LobbyUi_C" null ServerName))
  (bind _output_get (set `self.LobbyMenueWD` _returnvalue))
  (`UserWidget.AddToViewport` _output_get 0)
  (`WidgetBlueprintLibrary.SetInputMode_GameAndUIEx` self _output_get))

(event `CallUpdate`
  (params (PlayerInfo :type "/Game/Blueprints/OtherBlueprints/PlayerInfo Structure") (`ChangeStatus?` :type Boolean))
  (bind _aslobby (cast `/Game/Blueprints/Gamemodes/Lobby` (`GameplayStatics.GetGameMode`) :!pure true))
  (set `self.PlayerSettings` PlayerInfo)
  (`/Game/Blueprints/Gamemodes/Lobby.ChooseCharacter` _aslobby self (`.MyCharacter_11_DDBF666D60894881896C7AE0ADB25345` (break `/Game/Blueprints/OtherBlueprints/PlayerInfo` (`self.PlayerSettings`))) `ChangeStatus?`)
  (`/Engine/EditorBlueprintResources/StandardMacros.IsValid` _aslobby
    (:`Is Valid`
      (`/Game/Blueprints/Gamemodes/Lobby.EveryoneUpdate` _aslobby))))

(event `UpdateAvailableCharacters`
  (params (AvailableCharacters :type "Array of Boolean"))
  (bind _lobbymenuewd (`self.LobbyMenueWD`))
  (set `self.AvailableCharacters` AvailableCharacters)
  (`/Engine/EditorBlueprintResources/StandardMacros.IsValid` _lobbymenuewd
    (:`Is Valid`
      (for (_array_element _array_index) (`/Game/Blueprints/Widgets/CharacterSelect.PlayerButtons` (`/Game/Blueprints/Widgets/LobbyUi.CharacterSelect` _lobbymenuewd))
        (`Widget.SetIsEnabled` _array_element (`|GetArrayItem` (`self.AvailableCharacters`) _array_index))))))

(event `AttemptAssignCharacter`
  (params (CharacterID :type Integer))
  (set `self.PreviousSelected` (`self.SelectedCharacter`))
  (set `self.SelectedCharacter` CharacterID)
  (`self.CharacterCheck`))

(event `AddPlayerInfo`
  (params (PlayerInfo :type "Array of /Game/Blueprints/OtherBlueprints/PlayerInfo Structure"))
  (bind _lobbymenuewd (`self.LobbyMenueWD`))
  (set `self.AllConnectedPlayers` PlayerInfo)
  (`/Engine/EditorBlueprintResources/StandardMacros.IsValid` _lobbymenuewd
    (:`Is Valid`
      (`/Game/Blueprints/Widgets/LobbyUi.ClearPlayer` _lobbymenuewd)
      (for _array_element (`self.AllConnectedPlayers`)
        (bind (_myplayername _mycharacter _myplayerstatus) (break `/Game/Blueprints/OtherBlueprints/PlayerInfo` _array_element))
        (`/Game/Blueprints/Widgets/LobbyUi.PlayerWindowUpdate` (`self.LobbyMenueWD`) (select `bool` (== "Host" _myplayerstatus) :`false` (make `/Game/Blueprints/OtherBlueprints/PlayerInfo` _myplayername _mycharacter _myplayerstatus) :`true` _array_element))))))

(event `AssignPlayer`
  (setmembers `/Game/Blueprints/OtherBlueprints/PlayerInfo` :`StructRef` (`self.PlayerSettings`) :`MyCharacter` (`self.SelectedCharacter`) :`MyPlayerStatus` "Ready")
  (`self.SaveGame`)
  (`self.CallUpdate` (`self.PlayerSettings`) true))

(event `UpdateLobbySettings`
  (params (MapName :type Text) (MapTime :type Text))
  (bind _lobbymenuewd (`self.LobbyMenueWD`))
  (set `/Game/Blueprints/Widgets/LobbyUi.MapName` MapName _lobbymenuewd)
  (set `/Game/Blueprints/Widgets/LobbyUi.MapTime` MapTime _lobbymenuewd))

(event `UpdateChatServer`
  (params (Text :type Text))
  (bind _output_get (set `self.ChatTexts` Text))
  (bind _aslobby (cast `/Game/Blueprints/Gamemodes/Lobby` (`GameplayStatics.GetGameMode`)))
  (for _array_element (`/Game/Blueprints/Gamemodes/Lobby.AllPlayerControllers` _aslobby)
    (bind _aslobby_controller (cast `/Game/Blueprints/Controllers/LobbyController` _array_element))
    (`self.GetChat` _aslobby_controller _output_get)))

(event `GetChat`
  (params (TextToSend :type Text))
  (`/Game/Blueprints/Widgets/LobbyUi.UpdateChat` (`self.LobbyMenueWD`) TextToSend))

(event `ShowLoadingScreen`
  (`Widget.RemoveFromParent` (`self.LobbyMenueWD`))
  (bind _returnvalue (`|CreateWidget` "/Game/Blueprints/Widgets/LoadingScreen.LoadingScreen_C" self))
  (`UserWidget.AddToViewport` _returnvalue 0))

(event `UpdateNumberOfPlayers`
  (params (CurrentPlayers :type Integer) (MaxPlayers :type Integer))
  (bind _lobbymenuewd (`self.LobbyMenueWD`))
  (`/Engine/EditorBlueprintResources/StandardMacros.IsValid` _lobbymenuewd
    (:`Is Valid`
      (set `/Game/Blueprints/Widgets/LobbyUi.PlayersDisplay` (`|FormatText` "{CurrentPlayers} of {MaxPlayers}" (`KismetTextLibrary.Conv_IntToText` CurrentPlayers) (`KismetTextLibrary.Conv_IntToText` MaxPlayers)) _lobbymenuewd))))

(event `self.ReceiveEndPlay`
  (params (EndPlayReason :type "EEndPlayReason Enum" :default "Destroyed"))
  (`DestroySessionCallbackProxy.DestroySession` self :!label _label))

(event `Kicked`
  (`GameplayStatics.OpenLevelBySoftObjectPtr` "/Game/Maps/MainMenue.MainMenue")
  (goto _label))

(fn `CharacterCheck`
  (bind _availablecharacters (`/Game/Blueprints/Gamemodes/Lobby.AvailableCharacters` (cast `/Game/Blueprints/Gamemodes/Lobby` (`GameplayStatics.GetGameMode`) :!pure true)))
  (if (== (`|GetArrayItem` _availablecharacters (`self.SelectedCharacter`)) true)
    (`KismetArrayLibrary.Array_Set` _availablecharacters (`self.PreviousSelected`) true)
    (`KismetArrayLibrary.Array_Set` _availablecharacters (`self.SelectedCharacter`))
    (`self.AssignPlayer`)))

(fn `LoadGame`
  (bind _returnvalue (`GameplayStatics.LoadGameFromSlot` (`self.PlayerSave`)))
  (bind _asplayer_save_game (cast `/Game/Blueprints/OtherBlueprints/PlayerSaveGame` _returnvalue))
  (bind (_myplayername _mycharacter _myplayerstatus) (break `/Game/Blueprints/OtherBlueprints/PlayerInfo` (`/Game/Blueprints/OtherBlueprints/PlayerSaveGame.S_PlayerInfo` _asplayer_save_game)))
  (setmembers `/Game/Blueprints/OtherBlueprints/PlayerInfo` :`StructRef` (`self.PlayerSettings`) :`MyPlayerName` _myplayername :`MyCharacter` _mycharacter :`MyPlayerStatus` _myplayerstatus))

(fn `SaveGame`
  (bind _playersavegame (`self.PlayerSaveGame`))
  (`/Engine/EditorBlueprintResources/StandardMacros.IsValid` null
    (:`Is Valid`
      (bind _returnvalue (`GameplayStatics.CreateSaveGameObject` "/Game/Blueprints/OtherBlueprints/PlayerSaveGame.PlayerSaveGame_C"))
      (set `self.PlayerSaveGame` _returnvalue)
      (set `/Game/Blueprints/OtherBlueprints/PlayerSaveGame.S_PlayerInfo` (`self.PlayerSettings`) _playersavegame)
      (`GameplayStatics.SaveGameToSlot` _playersavegame (`self.PlayerSave`)))))

(fn `SaveGameCheck`
  (bind _returnvalue (`GameplayStatics.DoesSaveGameExist` (`self.PlayerSave`)))
  (if _returnvalue
    (`self.LoadGame`)
    (`self.SaveGame`)
    (else
      (`self.SaveGame`))))

(fn `UserConstructionScript`)