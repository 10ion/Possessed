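; Lobby game mode that tracks joining and leaving players, spawns their pawns and starts the match by server travel.
; PostLogin sets up each LobbyController and possesses a Character_Bp at a random PlayerStart, while logout frees the character slot.
; EveryoneUpdate rebuilds the player list and pushes it, counts and character availability to every controller.
; Character choice and start blocking are stubs, and launch always loads FirstPersonExampleMap, ignoring map settings.
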(event `self.K2_OnLogout`
  (params (ExitingController :type "Controller Object Reference"))
  (bind _allplayercontrollers (`self.AllPlayerControllers`))
  (for (_array_element _array_index) _allplayercontrollers
    (if (== _array_element ExitingController)
      (break)))
  (bind _aslobby_controller (cast `/Game/Blueprints/Controllers/LobbyController` (`|GetArrayItem` _allplayercontrollers _array_index)))
  (`KismetArrayLibrary.Array_Set` (`self.AvailableCharacters`) (`/Game/Blueprints/Controllers/LobbyController.SelectedCharacter` _aslobby_controller) true)
  (`KismetArrayLibrary.Array_Remove` (`self.AllPlayerControllers`) _array_index)
  (`KismetArrayLibrary.Array_Remove` (`self.ConnectedPlayers`) _array_index)
  (`self.EveryoneUpdate`))

(event `ChooseCharacter`
  (params (PlayerController :type "PlayerController Object Reference") (CharacterClass :type Integer) (ChangeStatus :type Boolean)))

(event `LaunchTheGame`
  (`KismetSystemLibrary.ExecuteConsoleCommand` "servertravel FirstPersonExampleMap" (`GameplayStatics.GetPlayerController` 0)))

(event `YouHaveBeenKicked`
  (params (PlayerID :type Integer))
  (`/Game/Blueprints/Controllers/LobbyController.Kicked` (cast `/Game/Blueprints/Controllers/LobbyController` (`|GetArrayItem` (`self.AllPlayerControllers`) PlayerID) :!pure true)))

(event `AddToKickList`)

(event `CannotStartGame`)

(event `EveryoneUpdate`
  (bind _allplayercontrollers (`self.AllPlayerControllers`))
  (bind _returnvalue (`KismetArrayLibrary.Array_Length` (`self.AllPlayerControllers`)))
  (set `self.CurrentPlayers` _returnvalue)
  (if (> _returnvalue 0)
    (`KismetArrayLibrary.Array_Clear` (`self.ConnectedPlayers`))
    (for _array_element _allplayercontrollers
      (bind _aslobby_controller (cast `/Game/Blueprints/Controllers/LobbyController` _array_element))
      (`KismetArrayLibrary.Array_Add` (`self.ConnectedPlayers`) (`/Game/Blueprints/Controllers/LobbyController.PlayerSettings` _aslobby_controller))
      (`/Game/Blueprints/Controllers/LobbyController.UpdateNumberOfPlayers` _aslobby_controller (`self.CurrentPlayers`) (`self.Number Of Players`)))
    (for _array_element_2 _allplayercontrollers
      (bind _aslobby_controller_2 (cast `/Game/Blueprints/Controllers/LobbyController` _array_element_2))
      (`/Game/Blueprints/Controllers/LobbyController.AddPlayerInfo` _aslobby_controller_2 (`self.ConnectedPlayers`))
      (`/Game/Blueprints/Controllers/LobbyController.UpdateAvailableCharacters` _aslobby_controller_2 (`self.AvailableCharacters`))
      (`self.AddToKickList`))
    (for (_array_element_3 _array_index) (`self.ConnectedPlayers`)
      (bind ((`MyPlayerName_2_3CA7385A7C134E90B4A5A97CD7D63CB7` _myplayername) (`MyCharacter_11_DDBF666D60894881896C7AE0ADB25345` _mycharacter) (`MyPlayerStatus_8_01428A1CE0054A66B35CB11DCF1F1086` _myplayerstatus)) (break `/Game/Blueprints/OtherBlueprints/PlayerInfo` _array_element_3))
      (if (== _mycharacter -1)
        (`KismetArrayLibrary.Array_Set` (`self.ConnectedPlayers`) _array_index (make `/Game/Blueprints/OtherBlueprints/PlayerInfo` _myplayername _mycharacter _myplayerstatus))
        (set `self.CanStart?` true)
        (`self.CannotStartGame`)
        (else
          (set `self.CanStart?` true))))))

(event `ServerUpdateGameSettings`
  (params (MapName :type Text) (MapTime :type Text) (MapID :type Integer))
  (set `self.MapName` MapName)
  (set `self.MapTime` MapTime)
  (set `self.MapID` MapID)
  (for _array_element (`self.AllPlayerControllers`)
    (bind _aslobby_controller (cast `/Game/Blueprints/Controllers/LobbyController` _array_element))
    (`/Game/Blueprints/Controllers/LobbyController.UpdateLobbySettings` _aslobby_controller (`self.MapName`) (`self.MapTime`))))

(event `self.K2_PostLogin`
  (params (NewPlayer :type "PlayerController Object Reference"))
  (`/Engine/EditorBlueprintResources/ActorMacros.Switch Has Authority`
    (:`Authority`
      (`KismetArrayLibrary.Array_Add` (`self.AllPlayerControllers`) NewPlayer)
      (bind _outactors (`GameplayStatics.GetAllActorsOfClass` "/Script/Engine.PlayerStart"))
      (set `self.SpawnPoints` _outactors)
      (bind _asgame_info_instance (cast `/Game/Blueprints/OtherBlueprints/GameInfoInstance` (`GameplayStatics.GetGameInstance`)))
      (set `self.Server Name` (`/Game/Blueprints/OtherBlueprints/GameInfoInstance.Server Name` _asgame_info_instance))
      (set `self.Number Of Players` (`/Game/Blueprints/OtherBlueprints/GameInfoInstance.Number Of Players` _asgame_info_instance))
      (bind _aslobby_controller (cast `/Game/Blueprints/Controllers/LobbyController` NewPlayer))
      (`/Game/Blueprints/Controllers/LobbyController.InitialSetup` _aslobby_controller)
      (`/Game/Blueprints/Controllers/LobbyController.SetLobbyMenue` _aslobby_controller (`self.Server Name`))
      (`/Game/Blueprints/Controllers/LobbyController.UpdateLobbySettings` _aslobby_controller (`self.MapName`) (`self.MapTime`))
      (`self.Respawn Player` NewPlayer))))

(event `Respawn Player`
  (params (PlayerController :type "PlayerController Object Reference"))
  (bind _returnvalue (`Controller.K2_GetPawn` PlayerController))
  (bind _spawnpoints (`self.SpawnPoints`))
  (bind _output (`|GetArrayItem` _spawnpoints (`KismetMathLibrary.RandomIntegerInRange` 0 (- (`KismetArrayLibrary.Array_Length` _spawnpoints) 1))))
  (`/Engine/EditorBlueprintResources/StandardMacros.IsValid` _returnvalue
    (:`Is Valid`
      (`self.K2_DestroyActor` _returnvalue))
    (:`Is Not Valid`
      _))
  (bind _returnvalue_2 (`|SpawnActorFromClass` "/Game/Blueprints/Pawns/Character_Bp.Character_Bp_C" (`self.GetTransform` _output) "Undefined" "OverrideRootScale" null null))
  (`Controller.Possess` PlayerController _returnvalue_2)
  (`self.EveryoneUpdate`)
  (`KismetSystemLibrary.PrintString` (`KismetSystemLibrary.GetDisplayName` _output) true true (struct :`G` 0.66 :`B` 1.0 :`A` 1.0) 100.0))

(fn `UserConstructionScript`)