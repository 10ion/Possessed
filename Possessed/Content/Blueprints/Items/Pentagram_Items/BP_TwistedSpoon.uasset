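; Interactable Twisted Spoon item, one of the Pentagram items, that adds one to an inventory slot quantity when interacted with.
; The Interact event finds every WG_Inventory widget, including nested ones, and calls UpdateQuantity on each one's first slot.
; It also increments WhichSlot per inventory slot, but that count does not select the updated slot.
; InteractState always returns false, and the item stays in place after interaction.
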(event `/Game/Blueprints/OtherBlueprints/BP_Interact_Interface.Interact`
  (`WidgetBlueprintLibrary.GetAllWidgetsOfClass` "/Game/Blueprints/Widgets/WG_Inventory.WG_Inventory_C" false)
  (for _array_element _
    (bind _inventoryslots (`/Game/Blueprints/Widgets/WG_Inventory.InventorySlots` _array_element))
    (for _ _inventoryslots
      (set `self.WhichSlot` (+ (`self.WhichSlot`) 1)))
    (`/Game/Blueprints/OtherBlueprints/BPFI_Inventory.UpdateQuantity` (`|GetArrayItem` _inventoryslots) 1)))

(fn `Interact`
  (return))

(fn `InteractState`
  (returns (InteractState :type Boolean))
  (return false))

(fn `UserConstructionScript`)