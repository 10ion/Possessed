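; Pentagram ritual actor that takes matching quest items from the player's inventory when the character overlaps its box.
; It scans WG_Inventory slots, and WhichItem maps each item name to an index that selects which item Blueprint to spawn.
; Spawned items are spaced around a circle using sine and cosine, with collision disabled, and removed from the inventory.
; WinCheck reports a non-ghost win to the GameMode once the circle holds ItemsNeeded items.
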(event `Add Item`)

(event `Key|E`
  (params (Key :type "Key Structure")))

(event `self.Box.OnComponentEndOverlap`
  (params (OverlappedComponent :type "PrimitiveComponent Object Reference") (OtherActor :type "Actor Object Reference") (OtherComp :type "PrimitiveComponent Object Reference") (OtherBodyIndex :type Integer)))

(event `self.Box.OnComponentBeginOverlap`
  (params (OverlappedComponent :type "PrimitiveComponent Object Reference") (OtherActor :type "Actor Object Reference") (OtherComp :type "PrimitiveComponent Object Reference") (OtherBodyIndex :type Integer) (bFromSweep :type Boolean) (SweepResult :type "HitResult Structure (by ref)"))
  (bind _itemindex (`self.ItemIndex`))
  (bind _returnvalue (* 360.0 (/ (+ (`self.Number of Items in Circle`) 1) (`self.Items Needed`))))
  (cast `/Game/Blueprints/Pawns/FirstPersonCharacter1` OtherActor)
  (bind _foundwidgets (`WidgetBlueprintLibrary.GetAllWidgetsOfClass` "/Game/Blueprints/Widgets/WG_Inventory.WG_Inventory_C" false))
  (for _array_element _foundwidgets
    _)
  (bind _inventoryslots (`/Game/Blueprints/Widgets/WG_Inventory.InventorySlots` _array_element))
  (for (_ _array_index) _inventoryslots
    (bind _information (`/Game/Blueprints/Widgets/WG_Inventory_Slot.Information` (`|GetArrayItem` _inventoryslots _array_index)))
    (bind _output_get (set `self.ItemName` (`.Name_9_78FD7AC849FA6952B32C41A665950DF6` (break `/Game/Blueprints/OtherBlueprints/ST_Item` _information))))
    (`self.WhichItem` _output_get)
    (if (`self.ItemFound`)
      (`KismetSystemLibrary.PrintString` (`KismetStringLibrary.Conv_IntToString` _itemindex))
      (bind _returnvalue_2 (`|SpawnActorFromClass` (select `int` _itemindex :`0` "/Game/Blueprints/Items/Pentagram_Items/BP_TwistedSpoon.BP_TwistedSpoon_C" :`1` "/Game/Blueprints/Items/Pentagram_Items/BP_StuffedBear.BP_StuffedBear_C" :`2` "/Game/Blueprints/Items/Pentagram_Items/BP_RabbitsFoot.BP_RabbitsFoot_C" :`3` "/Game/Blueprints/Items/Pentagram_Items/BP_DogCollar.BP_DogCollar_C" :`4` "/Game/Blueprints/Items/Pentagram_Items/BP_UsedCandle.BP_UsedCandle_C" :`5` "/Game/Blueprints/Items/Pentagram_Items/BP_UsedMatch.BP_UsedMatch_C" :`6` "/Game/Blueprints/Items/Pentagram_Items/BP_Journal.BP_Journal_C" :`7` "/Game/Blueprints/Items/Pentagram_Items/BP_OldCoin.BP_OldCoin_C" :`8` "/Game/Blueprints/Items/Pentagram_Items/BP_HairTies.BP_HairTies_C" :`9` "/Game/Blueprints/Items/Pentagram_Items/BP_RustyKnife.BP_RustyKnife_C" :`10` "/Game/Blueprints/Items/Pentagram_Items/BP_EmmaSkull.BP_EmmaSkull_C" :!type "Actor Class Reference") (`KismetMathLibrary.MakeTransform` (+ (`SceneComponent.K2_GetComponentLocation` (`self.Box`)) (* 100.0 (`KismetMathLibrary.MakeVector` (`KismetMathLibrary.DegCos` _returnvalue) (`KismetMathLibrary.DegSin` _returnvalue))))) "Undefined" "OverrideRootScale" null null))
      (`self.SetActorEnableCollision` _returnvalue_2 false)
      (set `self.Number of Items in Circle` (+ (`self.Number of Items in Circle`) 1))
      (set `self.ItemIndex` -1)
      (`/Game/Blueprints/OtherBlueprints/BPFI_Inventory.RemoveItem` _information))))

(event `UpdateList`
  (set `/Game/Blueprints/Pawns/FirstPersonCharacter1.NumberOfItemsCollected` (`self.Number of Items in Circle`) (cast `/Game/Blueprints/Pawns/FirstPersonCharacter1` (stale `self.Box.OnComponentBeginOverlap` OtherActor) :!pure true)))

(event `WinCheck`
  (if (== (`self.Number of Items in Circle`) (`self.Items Needed`))
    (message `/Game/Blueprints/OtherBlueprints/GameFinish.WhoWon` (`GameplayStatics.GetGameMode`) false true)))

(fn `SpawnLocation`)

(fn `UserConstructionScript`)

(fn `WhichItem`
  (params (Name :type Name))
  (for (_array_element _array_index) (`self.PentagramItemArray`)
    (if (== (`self.ItemName`) _array_element)
      (set `self.ItemIndex` _array_index)))
  (if (not (== (`self.ItemIndex`) -1))
    (set `self.ItemFound` true)
    (else
      (set `self.ItemFound` false))))